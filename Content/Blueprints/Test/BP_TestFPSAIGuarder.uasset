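; BP_TestFPSAIGuarder is a test AI guard that reacts to pawns it sees and noises it hears, and displays its state and health.
; Pawn sensing events pass straight to OnPawnSeen and OnNoiseHeard, whose logic is not defined in this graph.
; State and health change events update a WBP_GuardState widget, showing blank, "?" or "!" for idle, suspicious or alerted, plus health as text.
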(event OnSeePawn(PawnSensingComp)
  (params (Pawn :type Pawn%20Object%20Reference))
  (Class|FPSAIGuarder|OnPawnSeen Pawn))

(event OnHearNoise(PawnSensingComp)
  (params (Instigator :type Pawn%20Object%20Reference) (Location :type Vector%20%28by%20ref%29 :default "0, 0, 0") (Volume :type Float%20%28single-precision%29))
  (Class|FPSAIGuarder|OnNoiseHeard Instigator Location Volume))

(event EventBeginPlay)

(event Collision|EventActorBeginOverlap
  (params (OtherActor :type Actor%20Object%20Reference)))

(event EventTick
  (params (DeltaSeconds :type Float%20%28single-precision%29)))

(event EventOnStateChanged
  (params (NewState :type EAIGuardState%20Enum :default "Idle"))
  (bind _aswbp_guard_state (Utilities|Casting|CastToWBP_GuardState (UserInterface|GetUserWidgetObject (Variables|Default|GetWidget))))
  (Default|SetNewText _aswbp_guard_state (Utilities|Select :Index NewState :Idle "" :Suspicious "?" :Alerted "!")))

(event EventOnHealthChanged
  (params (heal :type Float%20%28single-precision%29))
  (bind _aswbp_guard_state (Utilities|Casting|CastToWBP_GuardState (UserInterface|GetUserWidgetObject (Variables|Default|GetWidget))))
  (Default|SetHealthText _aswbp_guard_state (Utilities|Text|ToText(Float) heal "HalfToEven")))

(fn ConstructionScript)