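; Player controller Blueprint that binds the chat window input to an OpenChatWindow call, whose implementation is not in this file.
; The rest of the event graph is disconnected and never runs.
; That unused logic covers toggling an animated chat widget with input mode and cursor switching, creating a game-over widget, and stopping AI guard movement.
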(event EventBeginPlay)

(event EventTick
  (params (DeltaSeconds :type Float%20%28single-precision%29)))

(event Input|ActionEvents|InputActionOpenChatWindow
  (params (Key :type Key%20Structure))
  ;[1 1 1] Open Chat Window
  (:Pressed
    (Class|FPSPlayerController|OpenChatWindow)))

(fn ConstructionScript)