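; BP_Guard is an AI guard that senses pawns by sight and sound and shows its alert state and health on a widget.
; PawnSensing events are forwarded to OnPawnSeen and OnNoiseHeard, whose logic lives outside this graph.
; OnStateChanged and OnHealthChanged update the WBP_GuardState widget with an idle, suspicious or alerted marker and a health readout.
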(event OnSeePawn(PawnSensingComp)
  (params (Pawn :type Pawn%20Object%20Reference))
  (Class|FPSAIGuard|OnPawnSeen Pawn))

(event OnHearNoise(PawnSensingComp)
  (params (Instigator :type Pawn%20Object%20Reference) (Location :type Vector%20%28by%20ref%29 :default "0, 0, 0") (Volume :type Float%20%28single-precision%29))
  (Class|FPSAIGuard|OnNoiseHeard Instigator Location Volume))

(event Custom|ChangedWidget
  (params (Value :type Float%20%28single-precision%29))
  (bind _aswbp_guard_state (Utilities|Casting|CastToWBP_GuardState (UserInterface|GetUserWidgetObject (Variables|Default|GetWidget))))
  (Default|SetHealthText _aswbp_guard_state (Utilities|Text|ToText(Float) Value "HalfToEven")))

(event EventBeginPlay)

(event Collision|EventActorBeginOverlap
  (params (OtherActor :type Actor%20Object%20Reference)))

(event EventTick
  (params (DeltaSeconds :type Float%20%28single-precision%29)))

(event EventOnStateChanged
  (params (NewState :type EAIState%20Enum :default "Idle"))
  (bind _aswbp_guard_state (Utilities|Casting|CastToWBP_GuardState (UserInterface|GetUserWidgetObject (Variables|Default|GetWidget))))
  (Default|SetNewText _aswbp_guard_state (Utilities|Select :Index NewState :Idle "" :Suspicious "?" :Alerted "!")))

(event EventOnHealthChanged
  (params (heal :type Float%20%28single-precision%29))
  (CallFunction|ChangedWidget heal))

(fn ConstructionScript)