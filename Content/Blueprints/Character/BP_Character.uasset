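; Character Blueprint holding disconnected prototype logic for an in-game chat system and first-person mesh visibility.
; CreateChat, BeginPlay and the construction script are empty, so none of the graph logic runs.
; Orphaned nodes create WBP_ChatSystem, add WBP_Message per BP_Player, and toggle animation, input mode and cursor.
; Other unwired fragments set owner visibility for first-person arms, gun and body meshes.
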(event EventCreateChat
  (params (PlayerController :type Player%20Controller%20Object%20Reference))
  ;[1 1 1] Create Chat
)

(event EventBeginPlay)

(event Input|ActionEvents|InputActionOpenChatWindow
  (params (Key :type Key%20Structure))
  ;[1 1 1] Input Open Chat Window
)

(fn ConstructionScript)