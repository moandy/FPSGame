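; Player Blueprint holding disconnected graph logic for multiplayer chat and first-person/third-person mesh visibility; none of it runs and the construction script is empty.
; The chat fragments create a chat widget shared with BP_FPSPlayerState, multicast messages into message widgets, and toggle the window's animation, input mode and cursor.
; The visibility fragments show first-person arms and gun to the owner while hiding the body and third-person gun.
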(fn ConstructionScript)